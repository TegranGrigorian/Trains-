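; Freight wagon Blueprint for the train vehicle system, extending a parent wagon class.
; Its rerail, collision, look-at, end-play, derail hologram and representation color overrides only forward to the parent implementation.
; Cargo impact handling, surface-based impact FX and SFX, unbind check and easter egg hooks are empty stubs, and the player-to-collision distance function returns zero.
; The construction script is empty, so the graphs add no behavior of their own.
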(event `self.ReceiveEndPlay`
  (params (EndPlayReason :type "EEndPlayReason Enum" :default "Destroyed"))
  (`parent.ReceiveEndPlay` EndPlayReason))

(event `self.ReceiveOnRerail`
  (`parent.ReceiveOnRerail`))

(event `CargoImpactOnSimulation`
  (params (HitComponent :type "PrimitiveComponent Object Reference") (OtherActor :type "Actor Object Reference") (OtherComp :type "PrimitiveComponent Object Reference") (NormalImpulse :type "Vector Structure") (Hit :type "HitResult Structure (by ref)")))

(event `self.ReceiveOnCollided`
  (params (withVehicle :type "FGRailroadVehicle Object Reference") (impactVelocity :type "Float (single-precision)") (isPrimaryEvent :type Boolean) (isDerailed :type Boolean))
  (`parent.ReceiveOnCollided` withVehicle impactVelocity isPrimaryEvent isDerailed))

(event `FGUseableInterface.StartIsLookedAt`
  (params (byCharacter :type "FGCharacterPlayer Object Reference") (state :type "UseState Structure (by ref)"))
  (`parent.StartIsLookedAt` byCharacter state))

(event `FGUseableInterface.StopIsLookedAt`
  (params (byCharacter :type "FGCharacterPlayer Object Reference") (state :type "UseState Structure (by ref)"))
  (`parent.StopIsLookedAt` byCharacter state))

(fn `CheckLocationForUnbind`)

(fn `DistanceBetweenPlayerAndCollision`
  (returns (NewParam :type "Float (double-precision)"))
  (return 0.0))

(fn `GetDefaultRepresentationColor`
  (returns (ReturnValue :type "LinearColor Structure"))
  (bind _returnvalue (`parent.GetDefaultRepresentationColor`))
  (return _returnvalue))

(fn `GetDerailHologramMesh`
  (returns (ReturnValue :type "StaticMesh Object Reference"))
  (bind _returnvalue (`parent.GetDerailHologramMesh`))
  (return _returnvalue))

(fn `GetLookAtDecription`
  (params (byCharacter :type "FGCharacterPlayer Object Reference") (state :type "UseState Structure (by ref)"))
  (returns (ReturnValue :type Text))
  (return (`parent.GetLookAtDecription` byCharacter state)))

(fn `PlayCargeFirstImpact`
  (params (ImpactVelocity :type "Float (double-precision)")))

(fn `PlayEasterEgg`)

(fn `PlayFXOnImpact`
  (params (ImpactForce :type "Float (double-precision)") (PhysSurface :type "EPhysicalSurface Enum" :default "SurfaceType_Default") (ImpactLocation :type "Vector Structure")))

(fn `PlaySFXDefaultImpact`
  (params (Location :type "Vector Structure") (ImpactForce :type "Float (double-precision)")))

(fn `PlaySFXOnImpact`
  (params (ImpactForce :type "Float (double-precision)") (ImpactLocation :type "Vector Structure")))

(fn `PlaySFXRockImpact`
  (params (Location :type "Vector Structure") (ImpactForce :type "Float (double-precision)")))

(fn `PlaySFXTreeImpact`
  (params (Location :type "Vector Structure") (ImpactForce :type "Float (double-precision)")))

(fn `UserConstructionScript`)
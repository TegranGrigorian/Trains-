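; HS locomotive train vehicle Blueprint, a child class that adds almost no logic of its own.
; Possession, camera, VFX, honk, rerail, collision, customization and look-at events forward straight to the parent, as do the derail hologram mesh and possession queries.
; Name update, honk multicast, impact and derail effects, validation checks and the construction script are empty stubs.
; Its only distinct result is a black default light color.
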(event `self.ReceiveBeginPlay`
  (`parent.ReceiveBeginPlay`))

(event `self.ReceiveUnpossessed`
  (params (OldController :type "Controller Object Reference"))
  (`parent.ReceiveUnpossessed` OldController))

(event `self.ReceivePossessed`
  (params (NewController :type "Controller Object Reference"))
  (`parent.ReceivePossessed` NewController))

(event `self.OnNameChanged`
  (`parent.OnNameChanged`))

(event `UpdateTrainName`)

(event `FGSignificanceInterface.GainedSignificance`
  (`parent.GainedSignificance`))

(event `FGSignificanceInterface.LostSignificance`
  (`parent.LostSignificance`))

(event `self.UpdateCamera`
  (params (DeltaTime :type "Float (single-precision)"))
  (`parent.UpdateCamera` DeltaTime))

(event `self.UpdateVFX`
  (`parent.UpdateVFX`))

(event `self.OnHonkBegin`
  (`parent.OnHonkBegin`))

(event `self.OnHonkEnd`
  (`parent.OnHonkEnd`))

(event `BeginHonk`
  (params (AllowAlternativeHonk :type Boolean)))

(event `EndHonk`)

(event `MulticastOnHonkShort`)

(event `MulticastOnHonkDanger`)

(event `self.HonkShort`
  (`parent.HonkShort`))

(event `self.HonkDanger`
  (`parent.HonkDanger`))

(event `self.ReceiveOnRerail`
  (`parent.ReceiveOnRerail`))

(event `self.ReceiveOnCollided`
  (params (withVehicle :type "FGRailroadVehicle Object Reference") (impactVelocity :type "Float (single-precision)") (isPrimaryEvent :type Boolean) (isDerailed :type Boolean))
  (`parent.ReceiveOnCollided` withVehicle impactVelocity isPrimaryEvent isDerailed))

(event `FGColorInterface.SetCustomizationData`
  (params (customizationData :type "FactoryCustomizationData Structure (by ref)"))
  (`parent.SetCustomizationData` customizationData))

(event `FGUseableInterface.StartIsLookedAt`
  (params (byCharacter :type "FGCharacterPlayer Object Reference") (state :type "UseState Structure (by ref)"))
  (`parent.StartIsLookedAt` byCharacter state))

(event `FGUseableInterface.StopIsLookedAt`
  (params (byCharacter :type "FGCharacterPlayer Object Reference") (state :type "UseState Structure (by ref)"))
  (`parent.StopIsLookedAt` byCharacter state))

(fn `CheckActorVelocity`)

(fn `CheckValidationForStop`)

(fn `DefaultLightColor`
  (returns (Value :type "Vector Structure"))
  (return (0.0 0.0 0.0)))

(fn `EasterEgg`
  (params (NewParam :type "Float (double-precision)")))

(fn `GetDerailHologramMesh`
  (returns (ReturnValue :type "StaticMesh Object Reference"))
  (bind _returnvalue (`parent.GetDerailHologramMesh`))
  (return _returnvalue))

(fn `IsPossessed`
  (returns (ReturnValue :type Boolean))
  (bind _returnvalue (`parent.IsPossessed`))
  (return _returnvalue))

(fn `PlayLocomotiveImpact&DerailSFX`
  (params (ImpactForce :type "Float (double-precision)")))

(fn `PlayLocomotiveImpactSFX`
  (params (ImpactForce :type "Float (double-precision)")))

(fn `SpawnCollisionVFX`
  (params (ImpactForceScale :type "Float (double-precision)")))

(fn `SpawnDeRailVFX`
  (params (Location :type "Vector Structure") (Velocity :type "Float (double-precision)") (ForwardVector :type "Vector Structure") (Surface :type "EPhysicalSurface Enum" :default "SurfaceType_Default")))

(fn `UserConstructionScript`)